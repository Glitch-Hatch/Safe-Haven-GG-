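; Spawner that lays a square grid of BP_BuildSlot actors around the world origin at BeginPlay, then hides each slot's highlight mesh.
; Helper functions derive cell steps and opposite corners from the slot class's default VBuildSize and BoxesFromMiddle.
; A while loop on Done spawns row by row from negative to positive corner, clearing the flag at the last.
; Both axes step by the Y width; BoxLengthCordChangeX goes unused.
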(event `self.ReceiveBeginPlay`
  (bind _boxes_from_middle (`self.Boxes from middle`))
  (bind _boxes_from_middle_2 (`self.Boxes from middle`))
  (set `self.BoxLength(cordChange)(X)` (`KismetMathLibrary.FTrunc` (.x (* (`.V_Build Size` (defaults `/Game/Code/Gathering_BPs/BP_BuildSlot` "/Game/Code/Gathering_BPs/BP_BuildSlot.BP_BuildSlot_C")) (200.0 200.0 1.0)))))
  (set `self.BoxWidth(coordChange)(Y)` (`KismetMathLibrary.FTrunc` (.y (* (`.V_Build Size` (defaults `/Game/Code/Gathering_BPs/BP_BuildSlot` "/Game/Code/Gathering_BPs/BP_BuildSlot.BP_BuildSlot_C")) (200.0 200.0 1.0)))))
  (bind _output_get (set `self.Negetive corner` (`KismetMathLibrary.MakeVector` (.x (* (* (`.V_Build Size` (defaults `/Game/Code/Gathering_BPs/BP_BuildSlot` "/Game/Code/Gathering_BPs/BP_BuildSlot.BP_BuildSlot_C")) (-200.0 -200.0 1.0)) (`KismetMathLibrary.MakeVector` (`KismetMathLibrary.Conv_IntToDouble` _boxes_from_middle) (`KismetMathLibrary.Conv_IntToDouble` _boxes_from_middle)))) (.y (* (* (`.V_Build Size` (defaults `/Game/Code/Gathering_BPs/BP_BuildSlot` "/Game/Code/Gathering_BPs/BP_BuildSlot.BP_BuildSlot_C")) (-200.0 -200.0 1.0)) (`KismetMathLibrary.MakeVector` (`KismetMathLibrary.Conv_IntToDouble` _boxes_from_middle) (`KismetMathLibrary.Conv_IntToDouble` _boxes_from_middle)))))))
  (set `self.Current Location` _output_get)
  (set `self.Positive corner` (`KismetMathLibrary.MakeVector` (.x (* (* (`.V_Build Size` (defaults `/Game/Code/Gathering_BPs/BP_BuildSlot` "/Game/Code/Gathering_BPs/BP_BuildSlot.BP_BuildSlot_C")) (200.0 200.0 1.0)) (`KismetMathLibrary.MakeVector` (`KismetMathLibrary.Conv_IntToDouble` _boxes_from_middle_2) (`KismetMathLibrary.Conv_IntToDouble` _boxes_from_middle_2) 1.0))) (.y (* (* (`.V_Build Size` (defaults `/Game/Code/Gathering_BPs/BP_BuildSlot` "/Game/Code/Gathering_BPs/BP_BuildSlot.BP_BuildSlot_C")) (200.0 200.0 1.0)) (`KismetMathLibrary.MakeVector` (`KismetMathLibrary.Conv_IntToDouble` _boxes_from_middle_2) (`KismetMathLibrary.Conv_IntToDouble` _boxes_from_middle_2) 1.0)))))
  (while (`self.Done`)
    (`|SpawnActorFromClass` "/Game/Code/Gathering_BPs/BP_BuildSlot.BP_BuildSlot_C" (`KismetMathLibrary.MakeTransform` (`self.Current Location`) (struct) (`.V_Build Size` (defaults `/Game/Code/Gathering_BPs/BP_BuildSlot` "/Game/Code/Gathering_BPs/BP_BuildSlot.BP_BuildSlot_C"))) "Undefined" "MultiplyWithRoot" null null)
    (if (== (`self.Current Location`) (`self.Positive corner`))
      (set `self.Done` false)
      (elif (== (.x (`self.Current Location`)) (.x (`self.Positive corner`)))
        (set `self.Current Location` (`KismetMathLibrary.MakeVector` (.x (`self.Negetive corner`)) (+ (.y (`self.Current Location`)) (`self.BoxWidth(coordChange)(Y)`))))
        (else
          (set `self.Current Location` (`KismetMathLibrary.MakeVector` (+ (.x (`self.Current Location`)) (`self.BoxWidth(coordChange)(Y)`)) (.y (`self.Current Location`)) (.z (`self.Current Location`))))))))
  (bind _outactors (`GameplayStatics.GetAllActorsOfClass` "/Game/Code/Gathering_BPs/BP_BuildSlot.BP_BuildSlot_C"))
  (for _array_element _outactors
    (`SceneComponent.SetVisibility` (`/Game/Code/Gathering_BPs/BP_BuildSlot.MeshHilight` _array_element) false false)))

(fn `UserConstructionScript`)