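; Parent Blueprint for a member pawn that can be moved and assigned to gather wood, stone or food.
; Gather events set a building type, then Gather either releases the held slot or searches for a free matching BP_BuildSlot, claims it and sends the member there via AIMoveTo.
; Interacting removes any open build UI and creates a member widget showing the current task.
; Failed gathering resets the task to Empty.
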(event `self.ReceiveBeginPlay`
  (`|AIMoveTo` self (0.0 0.0 0.0) null))

(event `Event Open Interact UI`
  (`KismetSystemLibrary.PrintString` "Interacted")
  (bind _outactors (`GameplayStatics.GetAllActorsOfClass` "/Game/Code/UI/BuildUI/BP_BuildUI.BP_BuildUI_C"))
  (for _array_element _outactors
    (bind _asbp_build_ui (cast `/Game/Code/UI/BuildUI/BP_BuildUI` _array_element :!pure true))
    (if (`/Game/Code/UI/BuildUI/BP_BuildUI.B_WidgetExists` _asbp_build_ui)
      (`/Game/Code/UI/BuildUI/BP_BuildUI.Event Build UI Removal` _asbp_build_ui)
      (break)))
  (bind _returnvalue (`|CreateWidget` "/Game/Code/Members/BP_MemberUI.BP_MemberUI_C"))
  (`UserWidget.AddToViewport` _returnvalue 0)
  (set `self.OR_MemberUI` _returnvalue)
  (switch `/Game/Code/UI/BuildUI/E_BuildingSelect` (`self.E_Interact`)
    (:`NewEnumerator0`
      (`TextBlock.SetText` (`/Game/Code/Members/BP_MemberUI.CurrentTask` (`self.OR_MemberUI`)) "Food"))
    (:`NewEnumerator1`
      (`TextBlock.SetText` (`/Game/Code/Members/BP_MemberUI.CurrentTask` (`self.OR_MemberUI`)) "Children"))
    (:`NewEnumerator2`
      (`TextBlock.SetText` (`/Game/Code/Members/BP_MemberUI.CurrentTask` (`self.OR_MemberUI`)) "Stone"))
    (:`NewEnumerator3`
      (`TextBlock.SetText` (`/Game/Code/Members/BP_MemberUI.CurrentTask` (`self.OR_MemberUI`)) "Wood"))
    (:`NewEnumerator4`
      (`TextBlock.SetText` (`/Game/Code/Members/BP_MemberUI.CurrentTask` (`self.OR_MemberUI`)) "Nothing"))))

(event `Event Move`
  (params (`Move Location` :type "Vector Structure"))
  (`|AIMoveTo` self `Move Location` null))

(event `Event Gather Wood`
  (set `self.E_Interact` "NewEnumerator3")
  (`self.Gather`))

(event `Event Gather Stone`
  (set `self.E_Interact` "NewEnumerator2")
  (`self.Gather`))

(event `Event Gather Food`
  (set `self.E_Interact` "NewEnumerator0")
  (`self.Gather`))

(event `Gather`
  (if (`self.Space Exists`)
    (`/Game/Code/Gathering_BPs/BP_BuildSlot.Event Left` (`self.Space Interacted`))
    (else
      (bind _outactors (`GameplayStatics.GetAllActorsOfClass` "/Game/Code/Gathering_BPs/BP_BuildSlot.BP_BuildSlot_C"))
      (for _array_element _outactors
        (bind _asbp_build_slot (cast `/Game/Code/Gathering_BPs/BP_BuildSlot` _array_element :!pure true))
        (if (`|EnumEquality` (`/Game/Code/Gathering_BPs/BP_BuildSlot.E_Building` _asbp_build_slot) (`self.E_Interact`))
          (if (not (`/Game/Code/Gathering_BPs/BP_BuildSlot.Is Interacted` _asbp_build_slot))
            (set `self.Space Interacted` _asbp_build_slot)
            (`/Game/Code/Gathering_BPs/BP_BuildSlot.Event Interacted` (`self.Space Interacted`))
            (`|AIMoveTo` self (`self.K2_GetActorLocation` (`self.Space Interacted`)) null
              (:`then`
                (set `self.Space Exists` true)
                (break))))))
      (if (`self.Space Exists`)
        (set `self.Space Exists` false)
        (else
          (`self.Event Unable To Gather`))))))

(event `Event Unable To Gather`
  (set `self.E_Interact` "NewEnumerator4"))

(fn `UserConstructionScript`)