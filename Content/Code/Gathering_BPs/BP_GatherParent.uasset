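; BP_GatherParent is the parent Blueprint for gatherable objects that the player interacts with to collect resources.
; Interacted finds the first BP_Inventory_UI actor, passes it this object's EInteractableType as the gather type and starts gathering there.
; Left sets that gather type to nothing to end the gathering timer.
; Both events swap the placeholder cube's material to show whether it is in use.
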(event `Event Left`
  ; Take the Player UI and set what it's gathering to nothing, immediately ending the Gathering timer
  (bind _outactors (`GameplayStatics.GetAllActorsOfClass` "/Game/Code/UI/BP_Inventory_UI.BP_Inventory_UI_C"))
  (for _array_element _outactors
    (set `self.OR_InventoryUI` _array_element)
    (break))
  (`|VariableSetRef` (`/Game/Code/UI/BP_Inventory_UI.E_GatherType` (`self.OR_InventoryUI`)) "NewEnumerator3")
  ; Visibly no longer interacting
  (`PrimitiveComponent.SetMaterial` (`self.PlaceHolderCube`) 0 "/Game/Code/M_GatherAlone.M_GatherAlone"))

(event `Event Interacted`
  ; Pull the referance for the player's User Interface, then set the enum to whatever the player is gathering and start the gather function within the player
  (bind _outactors (`GameplayStatics.GetAllActorsOfClass` "/Game/Code/UI/BP_Inventory_UI.BP_Inventory_UI_C"))
  (for _array_element _outactors
    (set `self.OR_InventoryUI` _array_element)
    (break))
  (`|VariableSetRef` (`/Game/Code/UI/BP_Inventory_UI.E_GatherType` (`self.OR_InventoryUI`)) (`self.E_InteractableType`))
  (`/Game/Code/UI/BP_Inventory_UI.Event Begin Gathering` (`self.OR_InventoryUI`))
  ; Visibly interacting
  (`PrimitiveComponent.SetMaterial` (`self.PlaceHolderCube`) 0 "/Game/Code/M_GatherInteracted.M_GatherInteracted"))

(fn `UserConstructionScript`)