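; BP_BuildSlot is a building plot that becomes a farm, quarry or lumbermill where the player gathers food, stone or wood.
; Buildstructure marks it built and uses EBuilding to set the resource type and mesh.
; Once built, Interacted and Left find the first BP_Inventory_UI actor, set its gather type and begin or end gathering.
; The construction script scales the building and highlight meshes by VBuildSize.
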(event `Event Build structure`
  (set `self.Is Built` true)
  (switch `/Game/Code/UI/BuildUI/E_BuildingSelect` (`self.E_Building`)
    (:`NewEnumerator0`
      (set `self.E_InteractableType` "NewEnumerator0")
      (`StaticMeshComponent.SetStaticMesh` (`self.Building Mesh`) "/Game/artmeshes/farmplot2.farmplot2"))
    (:`NewEnumerator2`
      (set `self.E_InteractableType` "NewEnumerator2")
      (`StaticMeshComponent.SetStaticMesh` (`self.Building Mesh`) "/Game/artmeshes/farmplot1.farmplot1"))
    (:`NewEnumerator3`
      (set `self.E_InteractableType` "NewEnumerator1")
      (`StaticMeshComponent.SetStaticMesh` (`self.Building Mesh`) "/Game/artmeshes/fence.fence"))))

(event `Event Left`
  ; Take the Player UI and set what it's gathering to nothing, immediately ending the Gathering timer
  (if (`self.Is Built`)
    (bind _outactors (`GameplayStatics.GetAllActorsOfClass` "/Game/Code/UI/StandardUI/BP_Inventory_UI.BP_Inventory_UI_C"))
    (for _array_element _outactors
      (set `self.OR_InventoryUI` _array_element)
      (break))
    (`|VariableSetRef` (`/Game/Code/UI/StandardUI/BP_Inventory_UI.E_GatherType` (`self.OR_InventoryUI`)) "NewEnumerator3")
    (`/Game/Code/UI/StandardUI/BP_Inventory_UI.Event End gather` (`self.OR_InventoryUI`))))

(event `Event Interacted`
  ; Pull the referance for the player's User Interface, then set the enum to whatever the player is gathering and start the gather function within the player
  (if (`self.Is Built`)
    (bind _outactors (`GameplayStatics.GetAllActorsOfClass` "/Game/Code/UI/StandardUI/BP_Inventory_UI.BP_Inventory_UI_C"))
    (for _array_element _outactors
      (set `self.OR_InventoryUI` _array_element)
      (break))
    (`|VariableSetRef` (`/Game/Code/UI/StandardUI/BP_Inventory_UI.E_GatherType` (`self.OR_InventoryUI`)) (`self.E_InteractableType`))
    (`/Game/Code/UI/StandardUI/BP_Inventory_UI.Event Begin Gathering` (`self.OR_InventoryUI`))))

(fn `UserConstructionScript`
  (`SceneComponent.SetRelativeScale3D` (`self.Building Mesh`) (`self.V_Build Size`))
  (`SceneComponent.SetRelativeScale3D` (`self.MeshHilight`) (`self.V_Build Size`)))